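; WeaponSlot is a Blueprint actor that displays one weapon at its own location, chosen by type: Blade, Rifle or Kunai.
; SetItem calls ClearItem to destroy any existing item, spawns the matching actor class at the slot's transform, stores it as SpawnedItem and snap-attaches it to DefaultSceneRoot.
; The Kunai type spawns a model-only variant, and the event graph and construction script are empty.
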(fn `ClearItem`
  (bind _spawneditem (`self.SpawnedItem`))
  (`/Engine/EditorBlueprintResources/StandardMacros.IsValid` _spawneditem
    (:`Is Valid`
      (`self.K2_DestroyActor` _spawneditem))))

(fn `SetItem`
  (params (Type :type "/Game/Character/Player_Naruto/WeaponList Enum" :default "NewEnumerator0"))
  (bind _returnvalue (`self.GetTransform`))
  (`self.ClearItem`)
  (switch `/Game/Character/Player_Naruto/WeaponList` Type
    (:`NewEnumerator0`
      (bind _returnvalue_2 (`|SpawnActorFromClass` "/Game/Blueprints/Blade.Blade_C" _returnvalue "Undefined" "OverrideRootScale" null null))
      (bind _output_get (set `self.SpawnedItem` _returnvalue_2)))
    (:`NewEnumerator1`
      (bind _returnvalue_3 (`|SpawnActorFromClass` "/Game/Blueprints/Rifle.Rifle_C" _returnvalue "Undefined" "OverrideRootScale" null null))
      (bind _output_get_2 (set `self.SpawnedItem` _returnvalue_3)))
    (:`NewEnumerator2`
      (bind _returnvalue_4 (`|SpawnActorFromClass` "/Game/Blueprints/Kunai_ModelOnly.Kunai_ModelOnly_C" _returnvalue "Undefined" "OverrideRootScale" null null))
      (bind _output_get_3 (set `self.SpawnedItem` _returnvalue_4))))
  (`self.K2_AttachToComponent` _output_get (`self.DefaultSceneRoot`) "None" "SnapToTarget" "SnapToTarget" "SnapToTarget" true)
  (`self.K2_AttachToComponent` _output_get_2 (`self.DefaultSceneRoot`) "None" "SnapToTarget" "SnapToTarget" "SnapToTarget" true)
  (`self.K2_AttachToComponent` _output_get_3 (`self.DefaultSceneRoot`) "None" "SnapToTarget" "SnapToTarget" "SnapToTarget" true))

(fn `UserConstructionScript`)
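; BreathCollision is a short-lived projectile actor with a growing sphere, apparently the collision volume for a breath attack.
; On BeginPlay it adds a projectile movement component and sets a three-second lifespan.
; Each Tick enlarges the sphere by an increment that rises with elapsed time, so growth accelerates and depends on frame rate.
; The actor overlap event is empty, so no hit response is handled here.
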(event `self.ReceiveActorBeginOverlap`
  (params (OtherActor :type "Actor Object Reference")))

(event `self.ReceiveBeginPlay`
  (`AddComponent|NODE_AddProjectileMovementComponent-0`)
  (`self.SetLifeSpan` 3.0))

(event `self.ReceiveTick`
  (params (DeltaSeconds :type "Float (single-precision)"))
  (bind _sphere (`self.Sphere`))
  (set `self.time` (+ DeltaSeconds (`self.time`)))
  (`SceneComponent.SetWorldScale3D` _sphere (+ (`SceneComponent.K2_GetComponentScale` _sphere) (* (+ (`self.time`) 1.0) 0.25))))

(fn `UserConstructionScript`)
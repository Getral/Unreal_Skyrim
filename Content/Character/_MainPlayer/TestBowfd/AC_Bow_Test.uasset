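; Bow combat component for MainPlayer, a test version that handles equipping, aiming, drawing and firing.
; Aiming switches the character to controller-facing rotation and spawns a socketed arrow, while bow state follows each phase.
; Firing launches the arrow toward a camera trace point, with strength from draw time, then re-aims and redraws after the release montage if still aiming.
; The draw timer is non-looping, so draw time increments once per draw.
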(event `self.ReceiveBeginPlay`
  (bind _asmain_player (cast `/Game/Character/_MainPlayer/MainPlayer` (`self.GetOwner`)))
  (set `self.Mainplayer Ref` _asmain_player)
  (set `self.Initial Rotation rate` (`CharacterMovementComponent.RotationRate` (`Character.CharacterMovement` (`self.Mainplayer Ref`)))))

(event `AimBegin`
  (bind _charactermovement (`Character.CharacterMovement` (`self.Mainplayer Ref`)))
  ;[1 1 1] Aim Bow
  (set `self.is Aiming` true)
  (set `CharacterMovementComponent.bOrientRotationToMovement` false _charactermovement)
  (set `CharacterMovementComponent.bUseControllerDesiredRotation` true _charactermovement)
  (set `CharacterMovementComponent.RotationRate` (`self.aim Rotation Rate`) _charactermovement)
  (set `/Game/Character/_MainPlayer/TestBowfd/BP_Bow_Test.Bow State` "NewEnumerator1" (`self.Bow Ref`))
  (`self.SpawnArrow`)
  (`self.OnAimBegin`))

(event `AimEnd`
  (bind _charactermovement (`Character.CharacterMovement` (`self.Mainplayer Ref`)))
  ;[1 1 1] Aim Bow
  (set `self.is Aiming` false)
  (`self.Drawn End`)
  (set `CharacterMovementComponent.bOrientRotationToMovement` true _charactermovement)
  (set `CharacterMovementComponent.bUseControllerDesiredRotation` false _charactermovement)
  (set `CharacterMovementComponent.RotationRate` (`self.Initial Rotation rate`) _charactermovement)
  (set `/Game/Character/_MainPlayer/TestBowfd/BP_Bow_Test.Bow State` "NewEnumerator0" (`self.Bow Ref`))
  (`self.DestroyArrow`)
  (`self.OnAimEnd`))

(event `Drawn Begin`
  ;[1 1 1] Drawn Bow
  (`self.Can Draw Bow`
    (:`Yes`
      (set `self.is Drawing Bow` true)
      (bind _returnvalue (`KismetSystemLibrary.K2_SetTimerDelegate` (delegate `Increment Draw Time`) (`self.Draw Increment Time`)))
      (set `self.Draw Bow Timer` _returnvalue)
      (set `/Game/Character/_MainPlayer/TestBowfd/BP_Bow_Test.Bow State` "NewEnumerator2" (`self.Bow Ref`)))))

(event `Increment Draw Time`
  ;[1 1 1] Drawn Bow
  (bind _output_get (set `self.Draw Time` (+ (`self.Draw Time`) (`self.Draw Increment Time`))))
  (`KismetSystemLibrary.PrintString` (`KismetStringLibrary.Conv_DoubleToString` _output_get)))

(event `Drawn End`
  ;[1 1 1] Drawn Bow
  (set `self.is Drawing Bow` false)
  (set `self.Draw Time` 1.0)
  (`KismetSystemLibrary.K2_ClearAndInvalidateTimerHandle` (`self.Draw Bow Timer`))
  (set `/Game/Character/_MainPlayer/TestBowfd/BP_Bow_Test.Bow State` "NewEnumerator0" (`self.Bow Ref`)))

(event `Fire Arrow Begin`
  ;[1 1 1] Fire Arrow
  (if (`self.is Drawing Bow`)
    (set `self.is Fire Arrow` true)
    (`self.Fire Aimed Arrow`)
    (`self.Drawn End`)
    (`|PlayMontage` (`Character.Mesh` (`self.Mainplayer Ref`)) (`self.Bow Shoot Release`)
      (:`OnCompleted`
        _)
      (:`OnInterrupted`
        _))
    (`self.Fire Arrow End`)))

(event `Fire Arrow End`
  ;[1 1 1] Fire Arrow
  (set `self.is Fire Arrow` false)
  (if (`self.is Aiming`)
    (`self.AimBegin`)
    (`self.Drawn Begin`)))

(fn `Calculate Aim Directoin`
  (returns (Derection :type "Vector Structure"))
  (bind _returnvalue (`Actor.GetComponentByClass` (`self.Mainplayer Ref`) "/Script/Engine.CameraComponent"))
  (bind _returnvalue_2 (`SceneComponent.K2_GetComponentLocation` _returnvalue))
  (bind (_outhit _returnvalue_3) (`KismetSystemLibrary.LineTraceSingle` _returnvalue_2 (+ _returnvalue_2 (* (`SceneComponent.GetForwardVector` _returnvalue) 10000.0)) "TraceTypeQuery1"))
  (bind _arrow_ref (`self.Arrow Ref`)
    (:`then`
      (bind (_bblockinghit _binitialoverlap _time _distance _location _impactpoint _normal _impactnormal _physmat _hitactor _hitcomponent _hitbonename _bonename _hititem _elementindex _faceindex _tracestart _traceend) (`GameplayStatics.BreakHitResult` _outhit))
      (return (`KismetMathLibrary.GetDirectionUnitVector` (`Actor.K2_GetActorLocation` _arrow_ref) (`KismetMathLibrary.SelectVector` _location _traceend _returnvalue_3))))
    (:`else`)))

(fn `DestroyArrow`
  (bind _arrow_ref (`self.Arrow Ref`)
    (:`then`
      (`Actor.K2_DestroyActor` _arrow_ref))
    (:`else`)))

(fn `Equiped Bow`
  (bind _returnvalue (`|SpawnActorFromClass` (`self.Bow Class`) (`KismetMathLibrary.MakeTransform` (0.0 0.0 0.0)) "Undefined" "OverrideRootScale" null null))
  (bind _output_get (set `self.Bow Ref` _returnvalue))
  (`Actor.K2_AttachToComponent` _output_get (`Character.Mesh` (`self.Mainplayer Ref`)) (`self.Bow Socket Name`) "SnapToTarget" "SnapToTarget" "SnapToTarget" true))

(fn `Fire Aimed Arrow`
  (bind _arrow_ref (`self.Arrow Ref`)
    (:`then`
      (`Actor.K2_DetachFromActor` _arrow_ref "KeepWorld" "KeepWorld" "KeepWorld")
      (bind _derection (`self.Calculate Aim Directoin`))
      (`/Game/Character/_MainPlayer/TestBowfd/BP_Arrow_Test.Fire` _arrow_ref _derection (`KismetMathLibrary.FClamp` (`KismetMathLibrary.NormalizeToRange` (`self.Draw Time`) 0.0 (`/Game/Character/_MainPlayer/TestBowfd/BP_Bow_Test.MaxDrawTime` (`self.Bow Ref`)))))
      (set `self.Arrow Ref` null))
    (:`else`)))

(fn `SpawnArrow`
  (bind _returnvalue (`|SpawnActorFromClass` "/Game/Character/_MainPlayer/TestBowfd/BP_Arrow_Test.BP_Arrow_Test_C" (`KismetMathLibrary.MakeTransform` (0.0 -0.0 0.0) (struct)) "Undefined" "OverrideRootScale" null null))
  (bind _output_get (set `self.Arrow Ref` _returnvalue))
  (`Actor.K2_AttachToComponent` _output_get (`Character.Mesh` (`self.Mainplayer Ref`)) (`self.Arrow Socket Name`) "SnapToTarget" "SnapToTarget" "SnapToTarget" true))